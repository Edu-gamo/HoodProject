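; Puzzle Blueprint that makes an object grabbable once it reaches a trigger.
; Each Tick, until the Do flag is set, it tests whether the Sphere's owning actor overlaps the Trigger's owning actor.
; On the first overlap it switches the Sphere's collision object type to PhysicsBody to allow pickup, sets Do and destroys the Trigger component.
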(event EventTick
  (params (DeltaSeconds :type Float%20%28single-precision%29))
  ;[1 1 1] Canviar el tipus de Colisió per poder agafar l'objecte
  (if (not (Variables|Default|Getdo))
    (if (Collision|IsOverlappingActor (Components|GetOwner (Variables|Default|GetSphere)) (Components|GetOwner (Variables|Default|GetTrigger)) :!class /Script/Engine.Actor)
      (Collision|SetCollisionObjectType (Variables|Default|GetSphere) "ECC_PhysicsBody")
      (Variables|Default|Setdo true)
      (Components|DestroyComponent (Variables|Default|GetTrigger)))))

(fn ConstructionScript)