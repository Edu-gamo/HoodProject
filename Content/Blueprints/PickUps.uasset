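; PickUps is a collectible actor that the first-person character picks up by pressing E while in range.
; Overlapping the PickUpTrigger component sets a CanPick flag and enables the actor's input for player 0, and leaving reverses both.
; Pressing E while the flag is set destroys the actor and prints a Spanish "collectible acquired" message, with no inventory or count update.
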(event OnComponentBeginOverlap(PickUpTrigger)
  (params (OverlappedComponent :type Primitive%20Component%20Object%20Reference) (OtherActor :type Actor%20Object%20Reference) (OtherComp :type Primitive%20Component%20Object%20Reference) (OtherBodyIndex :type Integer) (bFromSweep :type Boolean) (SweepResult :type Hit%20Result%20Structure%20%28by%20ref%29))
  (if (== (Utilities|GetClass OtherActor) "/Game/FirstPersonCPP/Blueprints/FirstPersonCharacter.FirstPersonCharacter_C")
    (Variables|Default|SetcanPick true)
    (Input|EnableInput (Game|GetPlayerController 0))))

(event OnComponentEndOverlap(PickUpTrigger)
  (params (OverlappedComponent :type Primitive%20Component%20Object%20Reference) (OtherActor :type Actor%20Object%20Reference) (OtherComp :type Primitive%20Component%20Object%20Reference) (OtherBodyIndex :type Integer))
  (if (== (Utilities|GetClass OtherActor) "/Game/FirstPersonCPP/Blueprints/FirstPersonCharacter.FirstPersonCharacter_C")
    (Variables|Default|SetcanPick false)
    (Input|DisableInput (Game|GetPlayerController 0))))

(event OnBeginCursorOver(PickUpTrigger)
  (params (TouchedComponent :type Primitive%20Component%20Object%20Reference)))

(event EventBeginPlay)

(event Collision|EventActorBeginOverlap
  (params (OtherActor :type Actor%20Object%20Reference)))

(event EventTick
  (params (DeltaSeconds :type Float%20%28single-precision%29)))

(event Input|KeyboardEvents|E
  (params (Key :type Key%20Structure))
  (:Pressed
    (if (Math|Boolean|Equal(Boolean) (Variables|Default|GetcanPick) true)
      (Actor|DestroyActor)
      (Development|PrintText "Coleccionable adquirdo"))))

(fn ConstructionScript)