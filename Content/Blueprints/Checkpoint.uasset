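; Checkpoint trigger actor that saves the player's position, shows tutorial text and can flag levels as completed.
; On box overlap, a FirstPersonCharacter's location becomes LastCheckPoint in myGameInstance, and the first true Lvl1–Lvl4 boolean sets its matching done flag.
; MyWidget stays hidden as a text source, copied into the player's TutoText.
; Any end overlap clears that text and destroys MyWidget.
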(event OnComponentBeginOverlap(Box)
  (params (OverlappedComponent :type Primitive%20Component%20Object%20Reference) (OtherActor :type Actor%20Object%20Reference) (OtherComp :type Primitive%20Component%20Object%20Reference) (OtherBodyIndex :type Integer) (bFromSweep :type Boolean) (SweepResult :type Hit%20Result%20Structure%20%28by%20ref%29))
  (bind _asfirst_person_character (Utilities|Casting|CastToFirstPersonCharacter OtherActor))
  (bind _asmy_game_instance (Utilities|Casting|CastTomyGameInstance (Game|GetGameInstance)))
  (Variables|/Game/Blueprints/myGameInstance.myGameInstance_C|SetlastCheckPoint _asmy_game_instance (Transformation|GetActorLocation _asfirst_person_character))
  (bind _asfirst_person_character_2 (Utilities|Casting|CastToFirstPersonCharacter (Game|GetPlayerCharacter 0)))
  (Variables|/Game/FirstPersonCPP/Blueprints/FirstPersonCharacter.FirstPersonCharacter_C|SetTutoText _asfirst_person_character_2 (Variables|/Script/HoodProject.MyWidgetComponent|GetText (Variables|Default|GetMyWidget)))
  (if (Variables|Default|GetLvl1)
    (Variables|/Game/Blueprints/myGameInstance.myGameInstance_C|SetisLvl1Done _asmy_game_instance true)
    (elif (Variables|Default|GetLvl2)
      (Variables|/Game/Blueprints/myGameInstance.myGameInstance_C|SetisLvl2Done _asmy_game_instance true)
      (elif (Variables|Default|GetLvl3)
        (Variables|/Game/Blueprints/myGameInstance.myGameInstance_C|SetisLvl3Done _asmy_game_instance true)
        (elif (Variables|Default|GetLvl4)
          (Variables|/Game/Blueprints/myGameInstance.myGameInstance_C|SetisLvl4Done _asmy_game_instance true))))))

(event OnComponentEndOverlap(Box)
  (params (OverlappedComponent :type Primitive%20Component%20Object%20Reference) (OtherActor :type Actor%20Object%20Reference) (OtherComp :type Primitive%20Component%20Object%20Reference) (OtherBodyIndex :type Integer))
  (bind _asfirst_person_character (Utilities|Casting|CastToFirstPersonCharacter (Game|GetPlayerCharacter 0)))
  (Variables|/Game/FirstPersonCPP/Blueprints/FirstPersonCharacter.FirstPersonCharacter_C|SetTutoText _asfirst_person_character "")
  (Components|DestroyComponent (Variables|Default|GetMyWidget)))

(event EventBeginPlay
  (Rendering|SetVisibility (Variables|Default|GetMyWidget) false false))

(fn ConstructionScript)