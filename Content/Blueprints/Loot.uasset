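; Collectible pickup actor that the player takes by pressing E while inside its collider.
; LootCollider overlaps with FirstPersonCharacter set the CanPick flag and enable or disable the actor's input.
; Tick polls that flag to show or hide MyWidget.
; Pressing E destroys the actor, increments the character's Colecinables counter and prints an acquisition message.
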(event OnComponentEndOverlap(LootCollider)
  (params (OverlappedComponent :type Primitive%20Component%20Object%20Reference) (OtherActor :type Actor%20Object%20Reference) (OtherComp :type Primitive%20Component%20Object%20Reference) (OtherBodyIndex :type Integer))
  ;[1 1 1] Loot
  (if (== (Utilities|GetClass OtherActor) "/Game/FirstPersonCPP/Blueprints/FirstPersonCharacter.FirstPersonCharacter_C")
    (Variables|Default|SetcanPick false)
    (Input|DisableInput (Game|GetPlayerController 0))))

(event OnComponentBeginOverlap(LootCollider)
  (params (OverlappedComponent :type Primitive%20Component%20Object%20Reference) (OtherActor :type Actor%20Object%20Reference) (OtherComp :type Primitive%20Component%20Object%20Reference) (OtherBodyIndex :type Integer) (bFromSweep :type Boolean) (SweepResult :type Hit%20Result%20Structure%20%28by%20ref%29))
  ;[1 1 1] Loot
  (if (== (Utilities|GetClass OtherActor) "/Game/FirstPersonCPP/Blueprints/FirstPersonCharacter.FirstPersonCharacter_C")
    (Variables|Default|SetcanPick true)
    (Input|EnableInput (Game|GetPlayerController 0))))

(event EventTick
  (params (DeltaSeconds :type Float%20%28single-precision%29))
  ;[1 1 1] Show Widget
  (if (Variables|Default|GetcanPick)
    (Rendering|SetVisibility (Variables|Default|GetMyWidget) true false)
    (else
      (Rendering|SetVisibility (Variables|Default|GetMyWidget) false false))))

(event Input|KeyboardEvents|E
  (params (Key :type Key%20Structure))
  ;[1 1 1] Loot
  (:Pressed
    (if (Math|Boolean|Equal(Boolean) (Variables|Default|GetcanPick) true)
      (Actor|DestroyActor)
      (bind _asfirst_person_character (Utilities|Casting|CastToFirstPersonCharacter (Game|GetPlayerCharacter 0)))
      (bind _result (Math|Integer|IncrementInt (Variables|/Game/FirstPersonCPP/Blueprints/FirstPersonCharacter.FirstPersonCharacter_C|GetColecinables _asfirst_person_character))
        (:%20%20
          (Variables|/Game/FirstPersonCPP/Blueprints/FirstPersonCharacter.FirstPersonCharacter_C|SetColecinables _asfirst_person_character _result)
          (Development|PrintText "Coleccionable adquirdo"))))))

(fn ConstructionScript)