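; Lever actor that the player pulls with E to raise a referenced set of bars (Barrotes).
; Trigger overlap with the first-person character toggles input and a prompt, mirrored to the character's TutoText.
; The first press rotates the arm, plays a sound and clears the tutorial text.
; Tick interpolates the bars above their starting position once pulled, or whenever the game instance marks level 1 done.
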(event OnComponentBeginOverlap(Trigger)
  (params (OverlappedComponent :type Primitive%20Component%20Object%20Reference) (OtherActor :type Actor%20Object%20Reference) (OtherComp :type Primitive%20Component%20Object%20Reference) (OtherBodyIndex :type Integer) (bFromSweep :type Boolean) (SweepResult :type Hit%20Result%20Structure%20%28by%20ref%29))
  ;[1 1 1] Begin/End Overlap w/ Char
  (Utilities|Casting|CastToFirstPersonCharacter OtherActor)
  (Variables|Default|SetCanActivate true)
  (Input|EnableInput (Game|GetPlayerController 0))
  (if (not (Variables|Default|GetHasRotated))
    (Rendering|SetVisibility (Variables|Default|GetMyWidget) true false)
    (bind _asfirst_person_character (Utilities|Casting|CastToFirstPersonCharacter (Game|GetPlayerCharacter 0)))
    (Variables|/Game/FirstPersonCPP/Blueprints/FirstPersonCharacter.FirstPersonCharacter_C|SetTutoText _asfirst_person_character (Variables|/Script/HoodProject.MyWidgetComponent|GetText (Variables|Default|GetMyWidget)))))

(event OnComponentEndOverlap(Trigger)
  (params (OverlappedComponent :type Primitive%20Component%20Object%20Reference) (OtherActor :type Actor%20Object%20Reference) (OtherComp :type Primitive%20Component%20Object%20Reference) (OtherBodyIndex :type Integer))
  ;[1 1 1] Begin/End Overlap w/ Char
  (Utilities|Casting|CastToFirstPersonCharacter OtherActor)
  (Variables|Default|SetCanActivate false)
  (Input|DisableInput (Game|GetPlayerController 0))
  (Rendering|SetVisibility (Variables|Default|GetMyWidget) false false)
  (bind _asfirst_person_character (Utilities|Casting|CastToFirstPersonCharacter (Game|GetPlayerCharacter 0)))
  (Variables|/Game/FirstPersonCPP/Blueprints/FirstPersonCharacter.FirstPersonCharacter_C|SetTutoText _asfirst_person_character ""))

(event EventTick
  (params (DeltaSeconds :type Float%20%28single-precision%29))
  ;[1 1 1] Movimiento Barrote
  (bind _asmy_game_instance (Utilities|Casting|CastTomyGameInstance (Game|GetGameInstance)))
  (if (Variables|/Game/Blueprints/myGameInstance.myGameInstance_C|GetisLvl1Done _asmy_game_instance)
    (Transformation|SetActorRelativeLocation (Variables|Default|GetBarrotes) (Math|Interpolation|VInterpTo (Transformation|GetActorLocation (Variables|Default|GetBarrotes)) (+ (Variables|Default|GetInitial%20Pos) "0, 0,175.000000") DeltaSeconds 2.0) :!label _label)
    (elif (Variables|Default|GetHasRotated)
      (goto _label))))

(event EventBeginPlay
  ;[1 1 1] Setters
  (Rendering|SetVisibility (Variables|Default|GetMyWidget) false false)
  (Variables|Default|SetInitial%20Pos (Transformation|GetActorLocation (Variables|Default|GetBarrotes))))

(event Input|KeyboardEvents|E
  (params (Key :type Key%20Structure))
  ;[1 1 1] E Pressed
  (:Pressed
    (if (Variables|Default|GetCanActivate)
      (if (not (Variables|Default|GetHasRotated))
        (Transformation|AddRelativeRotation (Variables|Default|GetBrazoPalanca) "0, 0,150.000000" false false)
        (Variables|Default|SetHasRotated true)
        (Rendering|SetVisibility (Actor|GetComponentbyClass (Variables|Default|GetBarrotes) "/Script/HoodProject.MyWidgetComponent") false false)
        (Audio|SpawnSoundatLocation "/Game/Musica/palanca_snd.palanca_snd" (Transformation|GetWorldLocation (Variables|Default|GetMyWidget)))
        (bind _asfirst_person_character (Utilities|Casting|CastToFirstPersonCharacter (Game|GetPlayerCharacter 0)))
        (Variables|/Game/FirstPersonCPP/Blueprints/FirstPersonCharacter.FirstPersonCharacter_C|SetTutoText _asfirst_person_character "")))))

(fn ConstructionScript)