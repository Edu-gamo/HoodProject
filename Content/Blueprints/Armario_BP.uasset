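; Wardrobe (Armario) Blueprint that slides aside when its book (Llibre) is no longer overlapping the Box component.
; BeginPlay caches the starting relative location, and Tick checks the overlap, then eases the wardrobe along local Y toward a fixed offset with VInterpTo.
; The activation sound spawns at the wardrobe on every moving frame until it is within tolerance of the target.
; No logic moves it back.
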(event EventBeginPlay
  (Variables|Default|SetinitialPos (Variables|/Script/Engine.SceneComponent|GetRelativeLocation (Variables|Default|Getarmario))))

(event EventTick
  (params (DeltaSeconds :type Float%20%28single-precision%29))
  (bind _armario (Variables|Default|Getarmario))
  (bind _initialpos (Variables|Default|GetinitialPos))
  (bind _returnvalue (+ _initialpos "0,150.000000, 0"))
  (bind _relativelocation (Variables|/Script/Engine.SceneComponent|GetRelativeLocation _armario))
  (if (not (Class|PrimitiveComponent|IsOverlappingComponent (Variables|Default|GetLlibre) (Variables|Default|GetBox)))
    (if (not (Math|Vector|Equal(Vector) _relativelocation _returnvalue 1e+01))
      (Transformation|SetRelativeLocation _armario (Math|Interpolation|VInterpTo _relativelocation _returnvalue DeltaSeconds 2.0) false false)
      (Audio|SpawnSoundatLocation "/Game/Musica/armarioActivo_snd.armarioActivo_snd" (Transformation|GetWorldLocation (Variables|Default|Getarmario))))))

(fn ConstructionScript)