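; Balanza_BP is a balance scale actor that tilts its arms as objects come into contact with either side.
; Begin overlaps on the left and right arms add the overlapping component's mass to that side's weight total and rotate BalanzaBrazos by a fixed step in opposite directions.
; The tilt ignores the accumulated weights: their comparison never runs, and nothing reverses weight or rotation when an overlap ends.
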(event OnComponentBeginOverlap(BrazoIzquierdo)
  (params (OverlappedComponent :type Primitive%20Component%20Object%20Reference) (OtherActor :type Actor%20Object%20Reference) (OtherComp :type Primitive%20Component%20Object%20Reference) (OtherBodyIndex :type Integer) (bFromSweep :type Boolean) (SweepResult :type Hit%20Result%20Structure%20%28by%20ref%29))
  (Variables|Default|SetPesoBrazoIzquierdo (+ (Physics|GetMass OtherComp) (Variables|Default|GetPesoBrazoIzquierdo)))
  (Transformation|AddRelativeRotation (Variables|Default|GetBalanza_Brazos) "2.000000, 0, 0" false false))

(event OnComponentBeginOverlap(BrazoDerecho)
  (params (OverlappedComponent :type Primitive%20Component%20Object%20Reference) (OtherActor :type Actor%20Object%20Reference) (OtherComp :type Primitive%20Component%20Object%20Reference) (OtherBodyIndex :type Integer) (bFromSweep :type Boolean) (SweepResult :type Hit%20Result%20Structure%20%28by%20ref%29))
  (Variables|Default|SetPesoBrazoDerecho (+ (Physics|GetMass OtherComp) (Variables|Default|GetPesoBrazoDerecho)))
  (Transformation|AddRelativeRotation (Variables|Default|GetBalanza_Brazos) "-2.000000, 0, 0" false false))

(event EventBeginPlay)

(event Collision|EventActorBeginOverlap
  (params (OtherActor :type Actor%20Object%20Reference)))

(fn ConstructionScript)