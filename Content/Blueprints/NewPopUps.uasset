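; NewPopUps is a trigger actor that shows a one-time text pop-up when the first-person character overlaps its collider.
; On overlap it disables the character's input, clears all widgets, shows a PopUps widget with the actor's Text, and enables its own input.
; Pressing Enter re-enables character input, swaps the pop-up for a fresh HUD widget and destroys the trigger.
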(event OnComponentBeginOverlap(Collider)
  (params (OverlappedComponent :type Primitive%20Component%20Object%20Reference) (OtherActor :type Actor%20Object%20Reference) (OtherComp :type Primitive%20Component%20Object%20Reference) (OtherBodyIndex :type Integer) (bFromSweep :type Boolean) (SweepResult :type Hit%20Result%20Structure%20%28by%20ref%29))
  (bind _asfirst_person_character (Utilities|Casting|CastToFirstPersonCharacter OtherActor))
  (Input|DisableInput _asfirst_person_character (Game|GetPlayerController 0))
  (Viewport|RemoveAllWidgets)
  (bind _returnvalue (UserInterface|CreateWidget "/Game/HUD/PopUps.PopUps_C"))
  (Variables|/Game/HUD/PopUps.PopUps_C|SetTextToDisplay _returnvalue (Variables|Default|GetText))
  (UserInterface|Viewport|AddtoViewport _returnvalue 0)
  (Input|EnableInput (Game|GetPlayerController 0)))

(event Input|KeyboardEvents|Enter
  (params (Key :type Key%20Structure))
  (:Pressed
    (bind _asfirst_person_character (Utilities|Casting|CastToFirstPersonCharacter (Game|GetPlayerCharacter 0)))
    (Input|EnableInput _asfirst_person_character (Game|GetPlayerController 0))
    (Viewport|RemoveAllWidgets)
    (bind _returnvalue (UserInterface|CreateWidget "/Game/HUD/HUD.HUD_C"))
    (UserInterface|Viewport|AddtoViewport _returnvalue 0)
    (Actor|DestroyActor)))

(fn ConstructionScript)