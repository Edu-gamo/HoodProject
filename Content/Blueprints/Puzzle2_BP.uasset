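; Puzzle actor with a ball that is highlighted while the first-person character is inside a box volume.
; Box overlaps toggle a ShowBall flag, and Tick enables the Sphere's custom depth rendering every frame while it is set; leaving the box turns it off.
; Separately, when the Trigger begins an overlap while touching the Sphere, the Sphere's collision object type switches to PhysicsBody.
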(event OnComponentBeginOverlap(Box)
  (params (OverlappedComponent :type Primitive%20Component%20Object%20Reference) (OtherActor :type Actor%20Object%20Reference) (OtherComp :type Primitive%20Component%20Object%20Reference) (OtherBodyIndex :type Integer) (bFromSweep :type Boolean) (SweepResult :type Hit%20Result%20Structure%20%28by%20ref%29))
  ;[1 1 1] Mostrar bola
  (Utilities|Casting|CastToFirstPersonCharacter OtherActor)
  (Variables|Default|SetshowBall true))

(event OnComponentEndOverlap(Box)
  (params (OverlappedComponent :type Primitive%20Component%20Object%20Reference) (OtherActor :type Actor%20Object%20Reference) (OtherComp :type Primitive%20Component%20Object%20Reference) (OtherBodyIndex :type Integer))
  ;[1 1 1] Mostrar bola
  (Utilities|Casting|CastToFirstPersonCharacter OtherActor)
  (Variables|Default|SetshowBall false)
  (Rendering|SetRenderCustomDepth (Variables|Default|GetSphere) false))

(event OnComponentBeginOverlap(Trigger)
  (params (OverlappedComponent :type Primitive%20Component%20Object%20Reference) (OtherActor :type Actor%20Object%20Reference) (OtherComp :type Primitive%20Component%20Object%20Reference) (OtherBodyIndex :type Integer) (bFromSweep :type Boolean) (SweepResult :type Hit%20Result%20Structure%20%28by%20ref%29))
  (bind _sphere (Variables|Default|GetSphere))
  ;[1 1 1] Canvi de tipus de collisio
  (if (Class|PrimitiveComponent|IsOverlappingComponent _sphere (Variables|Default|GetTrigger))
    (Collision|SetCollisionObjectType _sphere "ECC_PhysicsBody")))

(event EventTick
  (params (DeltaSeconds :type Float%20%28single-precision%29))
  ;[1 1 1] Mostrar bola
  (if (Variables|Default|GetshowBall)
    (Rendering|SetRenderCustomDepth (Variables|Default|GetSphere) true)))

(fn ConstructionScript)