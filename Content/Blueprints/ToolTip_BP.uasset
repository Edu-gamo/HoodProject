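; Tutorial tooltip actor that shows a text message when the first-person player character enters its trigger.
; BeginPlay copies ToolTipText into MyWidget; on overlap, while ShowAgain is set, it reveals MyWidget and copies the text to the character's TutoText.
; Leaving the trigger hides MyWidget, clears TutoText and sets ShowAgain to false, so the tip does not reappear on later entries.
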(event OnComponentBeginOverlap(Trigger)
  (params (OverlappedComponent :type Primitive%20Component%20Object%20Reference) (OtherActor :type Actor%20Object%20Reference) (OtherComp :type Primitive%20Component%20Object%20Reference) (OtherBodyIndex :type Integer) (bFromSweep :type Boolean) (SweepResult :type Hit%20Result%20Structure%20%28by%20ref%29))
  ;[1 1 1] Poner la visibilidad en TRUE
  (Utilities|Casting|CastToFirstPersonCharacter OtherActor)
  (if (Variables|Default|GetshowAgain)
    (Rendering|SetVisibility (Variables|Default|GetMyWidget) true false)
    (bind _asfirst_person_character (Utilities|Casting|CastToFirstPersonCharacter (Game|GetPlayerCharacter 0)))
    (Variables|/Game/FirstPersonCPP/Blueprints/FirstPersonCharacter.FirstPersonCharacter_C|SetTutoText _asfirst_person_character (Variables|/Script/HoodProject.MyWidgetComponent|GetText (Variables|Default|GetMyWidget)))))

(event OnComponentEndOverlap(Trigger)
  (params (OverlappedComponent :type Primitive%20Component%20Object%20Reference) (OtherActor :type Actor%20Object%20Reference) (OtherComp :type Primitive%20Component%20Object%20Reference) (OtherBodyIndex :type Integer))
  ;[1 1 1] Poner la visiblidad en FALSE
  (Utilities|Casting|CastToFirstPersonCharacter OtherActor)
  (Rendering|SetVisibility (Variables|Default|GetMyWidget) false false)
  (Variables|Default|SetshowAgain false)
  (bind _asfirst_person_character (Utilities|Casting|CastToFirstPersonCharacter (Game|GetPlayerCharacter 0)))
  (Variables|/Game/FirstPersonCPP/Blueprints/FirstPersonCharacter.FirstPersonCharacter_C|SetTutoText _asfirst_person_character ""))

(event EventBeginPlay
  ;[1 1 1] Init Texto
  (Variables|/Script/HoodProject.MyWidgetComponent|SetText (Variables|Default|GetMyWidget) (Variables|Default|GetToolTip%20Text)))

(fn ConstructionScript)