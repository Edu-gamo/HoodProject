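; Game instance that keeps an array of the world's Loot actors and reports each one's Collected value through debug prints.
; On Init it runs a check, which fills the array from all Loot actors whenever it is empty.
; The check then loops over the array, removing null entries and calling itself recursively after each removal, and prints the name and Collected value of the others.
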(event Custom|check
  (if (<= (Utilities|Array|Length (Variables|Default|Getcollected)) 0)
    (Development|PrintString "EMPTY")
    (bind _outactors (Actor|GetAllActorsOfClass "/Game/Blueprints/Loot.Loot_C"))
    (bind _output_get (Variables|Default|Setcollected _outactors))
    (else
      (Development|PrintString "NO EMPTY")))
  (for (_array_element _array_index) _output_get
    (if (== _array_element 0)
      (Utilities|Array|RemoveIndex (Variables|Default|Getcollected) _array_index)
      (CallFunction|Check)
      (else
        (Development|PrintString (Utilities|String|Append (Utilities|GetObjectName _array_element) " : " (Utilities|String|ToString(Boolean) (Variables|/Game/Blueprints/Loot.Loot_C|Getcollected _array_element))))))))

(event EventInit
  (CallFunction|Check))