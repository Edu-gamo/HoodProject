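; Puzzle chalice that raises a set of bars (Barrotes) while puzzle objects sit in its trigger and lowers them once it empties.
; Overlap events match "Puzzle" in object names to update a ball counter and movement flag.
; Tick stores the bars' initial height once, then steps them up to a fixed offset or back down.
; For puzzle instances, the game instance's level 4 completion flag forces upward movement, bypassing that limit.
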(event OnComponentBeginOverlap(TriggerCaliz)
  (params (OverlappedComponent :type Primitive%20Component%20Object%20Reference) (OtherActor :type Actor%20Object%20Reference) (OtherComp :type Primitive%20Component%20Object%20Reference) (OtherBodyIndex :type Integer) (bFromSweep :type Boolean) (SweepResult :type Hit%20Result%20Structure%20%28by%20ref%29))
  ;[1 1 1] Setters
  (if (Utilities|String|Contains (Utilities|GetObjectName OtherActor) "Puzzle")
    (Variables|Default|SetMove true)
    (Math|Integer|IncrementInt (Variables|Default|GetcontadorBolas))))

(event OnComponentEndOverlap(TriggerCaliz)
  (params (OverlappedComponent :type Primitive%20Component%20Object%20Reference) (OtherActor :type Actor%20Object%20Reference) (OtherComp :type Primitive%20Component%20Object%20Reference) (OtherBodyIndex :type Integer))
  ;[1 1 1] Setters
  (if (Utilities|String|Contains (Utilities|GetObjectName OtherActor) "Puzzle")
    (Variables|Default|SetMove false)
    (Math|Integer|DecrementInt (Variables|Default|GetcontadorBolas))))

(event Custom|Tick1
  ;[1 1 1] Movimiento
  (if (Variables|Default|GetisPuzzle)
    (bind _asmy_game_instance (Utilities|Casting|CastTomyGameInstance (Game|GetGameInstance)))
    (if (Variables|/Game/Blueprints/myGameInstance.myGameInstance_C|GetisLvl4Done _asmy_game_instance)
      (Transformation|SetActorRelativeLocation (Variables|Default|GetBarrotes) (Math|Interpolation|VInterpTo (Variables|/Script/Engine.SceneComponent|GetRelativeLocation (Variables|/Script/Engine.Actor|GetRootComponent (Variables|Default|GetBarrotes))) (+ (Variables|/Script/Engine.SceneComponent|GetRelativeLocation (Variables|/Script/Engine.Actor|GetRootComponent (Variables|Default|GetBarrotes))) "0, 0,2.000000") 0.0 0.0) :!label _label)
      (else
        (if (Variables|Default|GetMove) :!label _label_2
          (if (> (+ (Variables|Default|GetInitialPosBarrote) 225.0) (.Z (Math|Vector|BreakVector (Transformation|GetActorLocation (Variables|Default|GetBarrotes)))))
            (if (>= (Variables|Default|GetcontadorBolas) 1)
              (goto _label)))
          (elif (not (> (Variables|Default|GetInitialPosBarrote) (.Z (Math|Vector|BreakVector (Variables|/Script/Engine.SceneComponent|GetRelativeLocation (Variables|/Script/Engine.Actor|GetRootComponent (Variables|Default|GetBarrotes)))))))
            (if (== (Variables|Default|GetcontadorBolas) 0)
              (Transformation|SetActorRelativeLocation (Variables|Default|GetBarrotes) (Math|Interpolation|VInterpTo (Variables|/Script/Engine.SceneComponent|GetRelativeLocation (Variables|/Script/Engine.Actor|GetRootComponent (Variables|Default|GetBarrotes))) (+ (Variables|/Script/Engine.SceneComponent|GetRelativeLocation (Variables|/Script/Engine.Actor|GetRootComponent (Variables|Default|GetBarrotes))) "0, 0,-2.000000") 0.0 0.0)))))))
    (else
      (goto _label_2))))

(event EventTick
  (params (DeltaSeconds :type Float%20%28single-precision%29))
  (CallFunction|Tick1)
  (Utilities|FlowControl|DoOnce false
    (:Completed
      ;[1 1 1] Setter del InitialPosBarrote
      (Variables|Default|SetInitialPosBarrote (.Z (Math|Vector|BreakVector (Transformation|GetActorLocation (Variables|Default|GetBarrotes))))))))

(fn ConstructionScript)