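; Prison door that swings open when the first-person player stands in its trigger, optionally requiring that the character has keys.
; Overlap events track the player and clear CanOpen while a component with "metal" in its first material's name is inside.
; Tick checks these flags and plays one of two timelines, chosen by InverseOpen, to yaw both hinge components.
; No closing logic is present.
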(event OnComponentBeginOverlap(DoorTrigger)
  (params (OverlappedComponent :type Primitive%20Component%20Object%20Reference) (OtherActor :type Actor%20Object%20Reference) (OtherComp :type Primitive%20Component%20Object%20Reference) (OtherBodyIndex :type Integer) (bFromSweep :type Boolean) (SweepResult :type Hit%20Result%20Structure%20%28by%20ref%29))
  (if (== (Utilities|GetClass OtherActor) "/Game/FirstPersonCPP/Blueprints/FirstPersonCharacter.FirstPersonCharacter_C")
    (Variables|Default|SetplayerOnDoor true)
    (elif (Utilities|String|Contains (Utilities|GetObjectName (Rendering|Material|GetMaterial OtherComp 0)) "metal")
      (Variables|Default|SetcanOpen false))))

(event OnComponentEndOverlap(DoorTrigger)
  (params (OverlappedComponent :type Primitive%20Component%20Object%20Reference) (OtherActor :type Actor%20Object%20Reference) (OtherComp :type Primitive%20Component%20Object%20Reference) (OtherBodyIndex :type Integer))
  (if (== (Utilities|GetClass OtherActor) "/Game/FirstPersonCPP/Blueprints/FirstPersonCharacter.FirstPersonCharacter_C")
    (Variables|Default|SetplayerOnDoor false)
    (elif (Utilities|String|Contains (Utilities|GetObjectName (Rendering|Material|GetMaterial OtherComp 0)) "metal")
      (Variables|Default|SetcanOpen true))))

(event EventTick
  (params (DeltaSeconds :type Float%20%28single-precision%29))
  (if (and (Variables|Default|GetplayerOnDoor) (Variables|Default|GetcanOpen))
    (if (Variables|Default|GetneedKey)
      (bind _asfirst_person_character (Utilities|Casting|CastToFirstPersonCharacter (Game|GetPlayerCharacter 0)))
      (if (Variables|/Game/FirstPersonCPP/Blueprints/FirstPersonCharacter.FirstPersonCharacter_C|Getkeys _asfirst_person_character)
        (if (Variables|Default|GetinverseOpen) :!label _label
          (bind _doorrot (Timeline|Timeline_0 Play)
            (:Update
              (Transformation|SetRelativeRotation (Variables|Default|GetVisagra_Down2) (Math|Rotator|MakeRotator 0.0 0.0 _doorrot) false false)
              (Transformation|SetRelativeRotation (Variables|Default|GetVisagra_Up2) (Math|Rotator|MakeRotator 0.0 0.0 _doorrot) false false)))
          (else
            (bind _doorrot_2 (Timeline|Timeline_1 Play)
              (:Update
                (Transformation|SetRelativeRotation (Variables|Default|GetVisagra_Down2) (Math|Rotator|MakeRotator 0.0 0.0 _doorrot_2) false false)
                (Transformation|SetRelativeRotation (Variables|Default|GetVisagra_Up2) (Math|Rotator|MakeRotator 0.0 0.0 _doorrot_2) false false))))))
      (else
        (goto _label)))))

(fn ConstructionScript)